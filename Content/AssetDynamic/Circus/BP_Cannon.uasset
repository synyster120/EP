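; BP_Cannon is a circus cannon actor whose aim can be set through two rotation variables.
; The construction script applies CannonRoationZ as the yaw of the SceneCannon component and CannonRoationY as the pitch of SceneCannonBody.
; Each component keeps its other rotation axes, and the event graph holds no runtime logic.
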(event EventBeginPlay)

(event Collision|EventActorBeginOverlap
  (params (OtherActor :type Actor%20Object%20Reference)))

(event EventTick
  (params (DeltaSeconds :type Float%20%28single-precision%29)))

(fn ConstructionScript
  (bind _scenecannon (Variables|Default|GetSceneCannon))
  (bind _scenecannonbody (Variables|Default|GetSceneCannonBody))
  (bind _relativerotation (Variables|/Script/Engine.SceneComponent|GetRelativeRotation _scenecannon))
  (bind _relativerotation_2 (Variables|/Script/Engine.SceneComponent|GetRelativeRotation _scenecannonbody))
  (bind (_roll _pitch) (Math|Rotator|BreakRotator _relativerotation))
  (bind (_roll_2 _pitch_2 _yaw) (Math|Rotator|BreakRotator _relativerotation_2))
  (Utilities|FlowControl|Sequence
    (:then_0
      (Transformation|SetRelativeRotation (Variables|Default|GetSceneCannon) (Math|Rotator|MakeRotator _roll _pitch (Variables|Default|GetCannonRoationZ)) false false))
    (:then_1
      (Transformation|SetRelativeRotation (Variables|Default|GetSceneCannonBody) (Math|Rotator|MakeRotator _roll_2 (Variables|Default|GetCannonRoationY) _yaw) false false))))