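; BP_ChessDoor is a two-leaf door actor from the Chess assets, with left and right doors posed by rotation.
; The construction script sets the yaw of each door's scene component from its own rotation variable, keeping the existing roll and pitch.
; It has no runtime logic, as its event graph holds only disabled placeholder events.
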(event EventBeginPlay)

(event Collision|EventActorBeginOverlap
  (params (OtherActor :type Actor%20Object%20Reference)))

(event EventTick
  (params (DeltaSeconds :type Float%20%28single-precision%29)))

(fn ConstructionScript
  (bind _sceneleftdoor (Variables|Default|GetSceneLeftDoor))
  (bind _scenerightdoor (Variables|Default|GetSceneRightDoor))
  (bind _relativerotation (Variables|/Script/Engine.SceneComponent|GetRelativeRotation _scenerightdoor))
  (bind _relativerotation_2 (Variables|/Script/Engine.SceneComponent|GetRelativeRotation _sceneleftdoor))
  (bind (_roll _pitch) (Math|Rotator|BreakRotator _relativerotation))
  (bind (_roll_2 _pitch_2) (Math|Rotator|BreakRotator _relativerotation_2))
  (Utilities|FlowControl|Sequence
    (:then_0
      (Transformation|SetRelativeRotation (Variables|Default|GetSceneRightDoor) (Math|Rotator|MakeRotator _roll _pitch (Variables|Default|GetCheesDoorRightRotationZ)) false false))
    (:then_1
      (Transformation|SetRelativeRotation (Variables|Default|GetSceneLeftDoor) (Math|Rotator|MakeRotator _roll_2 _pitch_2 (Variables|Default|GetChessDoorLeftRotationZ)) false false))))