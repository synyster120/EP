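; Alchemy pot puzzle that opens a door when it holds the required mix of red and green potions.
; Sphere overlap reads the dropped item's class-default ItemID and increments its count in the TargetTags map, ignoring IDs not in the map.
; An exact red and green count plays LS_OpenDoor_Sequence, with debug prints when either check fails.
; OnItemRemoved decrements the count without rechecking, and an unconnected older logging version remains in the graph.
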(event OnComponentBeginOverlap(Sphere)
  (params (OverlappedComponent :type Primitive%20Component%20Object%20Reference) (OtherActor :type Actor%20Object%20Reference) (OtherComp :type Primitive%20Component%20Object%20Reference) (OtherBodyIndex :type Integer) (bFromSweep :type Boolean) (SweepResult :type Hit%20Result%20Structure%20%28by%20ref%29))
  (bind _targettags (Variables|Default|GetTargetTags))
  (bind _targettags_2 (Variables|Default|GetTargetTags))
  (bind (_value _returnvalue) (Utilities|Map|Find _targettags "Potion_Red"))
  (bind (_value_2 _returnvalue_2) (Utilities|Map|Find _targettags_2 "Potion_Green"))
  ;[1 0.1042 0.1042] Find - Potion ID - Plus counting
  (bind _asepdropped_item (Utilities|Casting|CastToEPDroppedItem OtherActor))
  (if (Utilities|IsValidClass (Variables|/Script/StarBoardMap.EPDroppedItem|GetOriginalItemClass _asepdropped_item))
    (if (.ReturnValue (Utilities|Map|Find (Variables|Default|GetTargetTags) (.ItemID (Utilities|GetClassDefaults (Variables|/Script/StarBoardMap.EPDroppedItem|GetOriginalItemClass _asepdropped_item)))))
      (Utilities|Map|Add (Variables|Default|GetTargetTags) (.ItemID (Utilities|GetClassDefaults (Variables|/Script/StarBoardMap.EPDroppedItem|GetOriginalItemClass _asepdropped_item))) (+ (.Value (Utilities|Map|Find (Variables|Default|GetTargetTags) (.ItemID (Utilities|GetClassDefaults (Variables|/Script/StarBoardMap.EPDroppedItem|GetOriginalItemClass _asepdropped_item))))) 1))
      ;[1 0.4196 0] Condition - Red Potion == 2
      (if (and (== _value 2) _returnvalue)
        ;[1 1 0] Condition - Green Potion == 1
        (if (and (== _value_2 1) _returnvalue_2)
          ;[0.7344 0.8149 1] Sequence Play
          (bind _returnvalue_3 (Sequencer|Player|CreateLevelSequencePlayer "/Game/AssetDynamic/Alchemy/LS_OpenDoor_Sequence.LS_OpenDoor_Sequence"))
          (Sequencer|Player|Play _returnvalue_3 :!class /Script/MovieScene.MovieSceneSequencePlayer)
          (else
            (Development|PrintString "Potion_Grren :: cound < 1" true true "(R=1.000000,G=0.998505,B=0.000000,A=1.000000)")))
        (else
          (Development|PrintString "Potion_Red :: cound < 2" true true "(R=1.000000,G=0.420886,B=0.000000,A=1.000000)"))))
    (else
      (Development|PrintString "get class defaults --- fail"))))

(event EventBeginPlay)

(event EventOnItemRemoved
  (params (RemovedItem :type Actor%20Object%20Reference))
  ;[1 0.1042 0.1042] Find - Potion ID - Minus counting
  (bind _asepdropped_item (Utilities|Casting|CastToEPDroppedItem RemovedItem))
  (if (Utilities|IsValidClass (Variables|/Script/StarBoardMap.EPDroppedItem|GetOriginalItemClass _asepdropped_item))
    (if (.ReturnValue (Utilities|Map|Find (Variables|Default|GetTargetTags) (.ItemID (Utilities|GetClassDefaults (Variables|/Script/StarBoardMap.EPDroppedItem|GetOriginalItemClass _asepdropped_item)))))
      (Utilities|Map|Add (Variables|Default|GetTargetTags) (.ItemID (Utilities|GetClassDefaults (Variables|/Script/StarBoardMap.EPDroppedItem|GetOriginalItemClass _asepdropped_item))) (- (.Value (Utilities|Map|Find (Variables|Default|GetTargetTags) (.ItemID (Utilities|GetClassDefaults (Variables|/Script/StarBoardMap.EPDroppedItem|GetOriginalItemClass _asepdropped_item))))) 1)))))

(fn ConstructionScript)